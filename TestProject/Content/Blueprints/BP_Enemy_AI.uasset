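; Enemy AI character that patrols around its spawn point, reacts to sight and noise, and dies from projectile hits.
; Tick retries random patrol moves, gated by CanStartPatroling, and destroys the actor at zero health.
; PawnSensing interrupts patrol: sight triggers a faster move to the player's current location, noise a move near the sound.
; BP_FirstPersonProjectile overlaps on the capsule reduce Health and refresh the WB_AIHealthBar widget.
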(event OnSeePawn(PawnSensing)
  (params (Pawn :type Pawn%20Object%20Reference))
  (Variables|Default|SetisSeengPlayer true)
  (Variables|Default|SetcanStartPatroling false)
  (CallFunction|FollowPlayer))

(event OnHearNoise(PawnSensing)
  (params (Instigator :type Pawn%20Object%20Reference) (Location :type Vector%20%28by%20ref%29 :default "0, 0, 0") (Volume :type Float%20%28single-precision%29))
  (Variables|Default|SetisHearSomething true)
  (Variables|Default|SetcanStartPatroling false)
  (bind _randomlocation (Class|NavigationSystemV1|GetRandomLocationinNavigableRadius Location 1e+03 0 0))
  (AI|AIMoveTo self _randomlocation 0 5.0 false
    (:OnSuccess
      (Variables|Default|SetcanStartPatroling true))))

(event OnComponentBeginOverlap(CapsuleComponent)
  (params (OverlappedComponent :type Primitive%20Component%20Object%20Reference) (OtherActor :type Actor%20Object%20Reference) (OtherComp :type Primitive%20Component%20Object%20Reference) (OtherBodyIndex :type Integer) (bFromSweep :type Boolean) (SweepResult :type Hit%20Result%20Structure%20%28by%20ref%29))
  (Utilities|Casting|CastToBP_FirstPersonProjectile OtherActor)
  (Variables|Default|SetHealth (- (Variables|Default|GetHealth) 1e+01))
  (CallFunction|UpdateHealthBar))

(event Custom|FollowPlayer
  (Variables|/Script/Engine.CharacterMovementComponent|SetMaxWalkSpeed (Variables|Character|GetCharacterMovement) 5e+02)
  (AI|AIMoveTo self (Transformation|GetActorLocation (Game|GetPlayerCharacter 0)) 0 7e+01 false
    (:OnSuccess
      (Utilities|FlowControl|Delay 1.0)
      (Variables|Default|SetcanStartPatroling true))))

(event Custom|MoveToRandomLocation
  (if (Variables|Default|GetcanStartPatroling)
    (Variables|Default|SetcanStartPatroling false)
    (bind _randomlocation (Class|NavigationSystemV1|GetRandomLocationinNavigableRadius (Variables|Default|GetStart%20Pos) 2e+03 0 0))
    (Variables|/Script/Engine.CharacterMovementComponent|SetMaxWalkSpeed (Variables|Character|GetCharacterMovement) 3e+02)
    (AI|AIMoveTo self _randomlocation 0 5.0 false
      (:OnSuccess
        (Variables|Default|SetcanStartPatroling true)))))

(event EventBeginPlay
  (Utilities|FlowControl|Sequence
    (:then_0
      (Variables|Default|SetStart%20Pos (Transformation|GetActorLocation)))
    (:then_1
      (CallFunction|MovetoRandomLocation))
    (:then_2
      (CallFunction|UpdateHealthBar))))

(event Collision|EventActorBeginOverlap
  (params (OtherActor :type Actor%20Object%20Reference)))

(event EventTick
  (params (DeltaSeconds :type Float%20%28single-precision%29))
  (CallFunction|MovetoRandomLocation)
  (if (<= (Variables|Default|GetHealth) 0.0)
    (Actor|DestroyActor)))

(fn ConstructionScript)

(fn UpdateHealthBar
  (bind _aswb_aihealth_bar (Utilities|Casting|CastToWB_AIHealthBar (UserInterface|GetUserWidgetObject (Variables|Default|GetHealthBAr))))
  (Variables|/Game/Blueprints/WB_AIHealthBar.WB_AIHealthBar_C|SetHealth _aswb_aihealth_bar (/ (Variables|Default|GetHealth) 1e+02))
  (return))